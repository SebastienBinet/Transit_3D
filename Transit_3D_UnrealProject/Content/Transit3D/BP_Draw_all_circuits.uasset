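; Actor that draws all Transit3D circuits from a map of data tables, driven by an editor tick event.
; The construction script adds a child actor, then gives each table a circuit-holder component with its own custom mesh component.
; Transit3DEditorTick has each stored component draw its table.
; The in-actor functions that built quad-section tube triangles from table rows are disconnected leftovers.
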(event EventBeginPlay)

(event Collision|EventActorBeginOverlap
  (params (OtherActor :type Actor%20Object%20Reference)))

(event EventTransit3DEditorTick
  ;[1 1 1] Based on https://dev.epicgames.com/community/learning/tutorials/PBnR/creating-an-editor-tick-in-unreal-engine
  (Development|PrintString "ddssaa2")
  (bind _keys (Utilities|Map|Keys (Variables|Default|GetSB_DataTablesToDiplay)))
  (for _array_element _keys
    (if (.ReturnValue (Utilities|Map|Find (Variables|Default|GetSB_DataTablesToDiplay) _array_element))
      (Default|DrawThisDataTable (.Value (Utilities|Map|Find (Variables|Default|GetSB_DataTablesToDiplay) _array_element)) _array_element)
      (else
        (Development|PrintString "ERROr rerere1234" true true "(R=1.000000,G=0.023286,B=0.000000,A=1.000000)")))))

(fn ConstructionScript
  (Utilities|FlowControl|Sequence
    (:then_0
      (AddComponent|AddChildActorComponent false))
    (:then_2
      (bind _keys (Utilities|Map|Keys (Variables|Default|GetSB_DataTablesToDiplay)))
      (for _array_element _keys
        (bind _returnvalue (AddComponent|AddBPActorComponenttoHoldACircuit))
        (Utilities|Map|Add (Variables|Default|GetSB_DataTablesToDiplay) _array_element _returnvalue)
        (bind _returnvalue_2 (AddComponent|AddCustomMeshComponent false))
        (Default|AssignCustomMeshtoUsetoDraw _returnvalue _returnvalue_2)))))

(fn TestwithDTMesh03615h12Csv
  (params (MyDynamicMesh :type Dynamic%20Mesh%20Object%20Reference)))

(fn GetandAddOtherRowsOfDt)

(fn GetFirstRowOfDt)