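; Obsolete GeneratedDynamicMeshActor test Blueprint for experimenting with Geometry Script mesh editing.
; On rebuild, TestWithSinwWave appends a box, adds and moves a vertex, prints vertex positions and triangle indices, then deletes a triangle.
; It also sets one triangle on a separate CustomMesh component.
; Despite the function name, no sine wave is computed, and several triangle-editing experiments are left unconnected.
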(event EventBeginPlay)

(event Collision|EventActorBeginOverlap
  (params (OtherActor :type Actor%20Object%20Reference)))

(event EventTick
  (params (DeltaSeconds :type Float%20%28single-precision%29)))

(event Events|EventOnRebuildGeneratedMesh
  (params (TargetMesh :type Dynamic%20Mesh%20Object%20Reference))
  (CallFunction|TestwithSinwWave TargetMesh))

(fn ConstructionScript)

(fn TestwithSinwWave
  (params (MyDynamicMesh :type Dynamic%20Mesh%20Object%20Reference))
  (bind _output_get (Variables|Default|SetMyDynamicMesh MyDynamicMesh))
  (Class|GeometryScriptLibraryMeshPrimitiveFunctions|AppendBox :TargetMesh _output_get :Debug 0)
  (Utilities|FlowControl|Sequence
    (:then_0
      (bind _returnvalue (Class|GeometryScriptLibraryMeshBasicEditFunctions|AddVertextoMesh (Variables|Default|GetMyDynamicMesh) "200.000000,200.000000,200.000000" false))
      (Class|GeometryScriptLibraryMeshBasicEditFunctions|SetVertexPosition (Variables|Default|GetMyDynamicMesh) 6 "75.000000,75.000000,150.000000" false)
      (bind _positionlist (GeometryScript|MeshQueries|GetAllVertexPositions (Variables|Default|GetMyDynamicMesh)))
      (for _index (range 0 (Class|GeometryScriptLibraryListUtilityFunctions|GetVectorListLastIndex _positionlist))
        (Development|PrintString (Utilities|String|Append "xxx:" (Utilities|String|ToString(Integer) _index) " : " (Utilities|String|ToString(Vector) (.ReturnValue (Class|GeometryScriptLibraryListUtilityFunctions|GetVectorListItem _positionlist _index)))))))
    (:then_1
      (bind _trianglelist (Class|GeometryScriptLibraryMeshQueryFunctions|GetAllTriangleIndices (Variables|Default|GetMyDynamicMesh) false))
      (for _index_2 (range 0 (Class|GeometryScriptLibraryListUtilityFunctions|GetTriangleListLastTriangle _trianglelist))
        (Development|PrintString (Utilities|String|Append "xxx:" (Utilities|String|ToString(Integer) _index_2) " - " (Utilities|String|ToString(Integer) (.ReturnValue (Class|GeometryScriptLibraryListUtilityFunctions|GetTriangleListItem _trianglelist _index_2)))))))
    (:then_2
      (Class|GeometryScriptLibraryMeshBasicEditFunctions|DeleteTrianglefromMesh (Variables|Default|GetMyDynamicMesh) 0 false))
    (:then_3
      (Class|CustomMeshComponent|SetCustomMeshTriangles (Variables|Default|GetCustomMesh) (Utilities|Array|MakeArray (Utilities|Struct|MakeCustomMeshTriangle "0.000000,200.000000,200.000000" "200.000000,200.000000,200.000000" "0.000000,150.000000,200.000000"))))))