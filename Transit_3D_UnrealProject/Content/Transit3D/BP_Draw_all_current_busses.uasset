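; Work-in-progress Transit3D actor meant to draw current buses from a data table.
; On its Transit3DEditorTick event it prints a debug string, caches the StaticMeshActor whose display name is TestBusActor, and reads row "0" of the current-bus table.
; The spawn and move nodes that would use that row's XYZ are disconnected, so no bus is placed or moved.
; The construction script just adds a child actor component.
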(event EventBeginPlay)

(event Collision|EventActorBeginOverlap
  (params (OtherActor :type Actor%20Object%20Reference)))

(event EventTick
  (params (DeltaSeconds :type Float%20%28single-precision%29)))

(event EventTransit3DEditorTick
  (Development|PrintString "Hello 77777777777777777777777777777777777777777777777777")
  (Utilities|FlowControl|Sequence
    (:then_0
      (bind _outactors (Actor|GetAllActorsOfClass "/Script/Engine.StaticMeshActor"))
      (for _array_element _outactors
        (if (Utilities|Enum|Equal(Enum) (Utilities|GetDisplayName _array_element) "TestBusActor")
          (Variables|Default|SetTestBusActorVar _array_element))))
    (:then_1
      (bind _returnvalue (Utilities|GetDataTableRow (Variables|Default|GetSB_DataTableCurrentBussesInfoToDisplay) "0")))))

(fn ConstructionScript
  (AddComponent|AddChildActorComponent false))