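; Actor component that draws a transit circuit from a DataTable as a 3D tube, with time on the Z axis.
; DrawThisDataTable clears the triangle list, seeds four corner vertices from the first row, then stitches each row to the previous one with eight side triangles.
; The result goes to an assigned CustomMeshComponent.
; The DynamicMesh triangle deletion is ineffective because that reference is set to None first.
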(event Custom|Draw%20This%20Data%20Table
  (params (DataTableToDraw :type Data%20Table%20Object%20Reference))
  (Variables|Default|SetSB_DataTableToDraw DataTableToDraw)
  (Development|PrintString (Utilities|String|Append "Draw This Data Table: " (Utilities|GetDisplayName (Variables|Default|GetSB_DataTableToDraw))))
  (Variables|Default|SetMyDynamicMesh 0)
  (Utilities|FlowControl|Sequence
    (:then_0
      (Utilities|Array|Clear (Variables|Default|GetSB_Triangles)))
    (:then_1
      (Development|PrintString (Utilities|String|Append "There were " (Utilities|String|ToString(Integer) (Class|DynamicMesh|GetTriangleCount (Variables|Default|GetMyDynamicMesh))) "Triangles"))
      ;[1 1 1] Delete previous triangles
      (for _index (range (Class|DynamicMesh|GetTriangleCount (Variables|Default|GetMyDynamicMesh)) 0)
        (Class|GeometryScriptLibraryMeshBasicEditFunctions|DeleteTrianglefromMesh (Variables|Default|GetMyDynamicMesh) _index false)))
    (:then_2
      (CallFunction|GetFirstRowOfDt))
    (:then_3
      (CallFunction|GetandAddOtherRowsOfDt))
    (:then_4)
    (:then_5
      (Class|CustomMeshComponent|SetCustomMeshTriangles (Variables|Default|GetSB_AssignedCustomMeshComponent) (Variables|Default|GetSB_Triangles)))))

(event EventBeginPlay)

(event EventTick
  (params (DeltaSeconds :type Float%20%28single-precision%29)))

(fn GetandAddOtherRowsOfDt
  (bind _outrownames (DataTable|GetDataTableRowNames (Variables|Default|GetSB_DataTableToDraw)))
  (for _array_element _outrownames
    (Development|PrintString (Utilities|String|ToString(Name) _array_element))
    (bind _returnvalue (Utilities|GetDataTableRow (Variables|Default|GetSB_DataTableToDraw) _array_element)
      (:then
        (Utilities|FlowControl|Sequence
          (:then_1
            (Utilities|Array|AppendArray (Variables|Default|GetSB_Triangles) (Utilities|Array|MakeArray (Utilities|Struct|MakeCustomMeshTriangle (Utilities|Array|Get(acopy) (Variables|Default|GetVerticesPreviousDtRow)) (Utilities|Array|Get(acopy) (Variables|Default|GetVerticesPreviousDtRow) 1) (Math|Vector|MakeVectorNetQuantize (.TopFastLeftX (Utilities|Struct|BreakS_Transit3DFourVerticesOfATime _returnvalue)) (.TopFastLeftY (Utilities|Struct|BreakS_Transit3DFourVerticesOfATime _returnvalue)) (.TopFastLeftTimeZ (Utilities|Struct|BreakS_Transit3DFourVerticesOfATime _returnvalue)))) (Utilities|Struct|MakeCustomMeshTriangle (Math|Vector|MakeVectorNetQuantize (.TopFastLeftX (Utilities|Struct|BreakS_Transit3DFourVerticesOfATime _returnvalue)) (.TopFastLeftY (Utilities|Struct|BreakS_Transit3DFourVerticesOfATime _returnvalue)) (.TopFastLeftTimeZ (Utilities|Struct|BreakS_Transit3DFourVerticesOfATime _returnvalue))) (Utilities|Array|Get(acopy) (Variables|Default|GetVerticesPreviousDtRow) 1) (Math|Vector|MakeVectorNetQuantize (.TopFastRightX (Utilities|Struct|BreakS_Transit3DFourVerticesOfATime _returnvalue)) (.TopFastRightY (Utilities|Struct|BreakS_Transit3DFourVerticesOfATime _returnvalue)) (.TopFastRightTimeZ (Utilities|Struct|BreakS_Transit3DFourVerticesOfATime _returnvalue)))) (Utilities|Struct|MakeCustomMeshTriangle (Utilities|Array|Get(acopy) (Variables|Default|GetVerticesPreviousDtRow) 1) (Utilities|Array|Get(acopy) (Variables|Default|GetVerticesPreviousDtRow) 2) (Math|Vector|MakeVectorNetQuantize (.TopFastRightX (Utilities|Struct|BreakS_Transit3DFourVerticesOfATime _returnvalue)) (.TopFastRightY (Utilities|Struct|BreakS_Transit3DFourVerticesOfATime _returnvalue)) (.TopFastRightTimeZ (Utilities|Struct|BreakS_Transit3DFourVerticesOfATime _returnvalue)))) (Utilities|Struct|MakeCustomMeshTriangle (Math|Vector|MakeVectorNetQuantize (.TopFastRightX (Utilities|Struct|BreakS_Transit3DFourVerticesOfATime _returnvalue)) (.TopFastRightY (Utilities|Struct|BreakS_Transit3DFourVerticesOfATime _returnvalue)) (.TopFastRightTimeZ (Utilities|Struct|BreakS_Transit3DFourVerticesOfATime _returnvalue))) (Utilities|Array|Get(acopy) (Variables|Default|GetVerticesPreviousDtRow) 2) (Math|Vector|MakeVectorNetQuantize (.BottomSlowRightX (Utilities|Struct|BreakS_Transit3DFourVerticesOfATime _returnvalue)) (.BottomSlowRightY (Utilities|Struct|BreakS_Transit3DFourVerticesOfATime _returnvalue)) (.BottomSlowRightTimeZ (Utilities|Struct|BreakS_Transit3DFourVerticesOfATime _returnvalue)))) (Utilities|Struct|MakeCustomMeshTriangle (Utilities|Array|Get(acopy) (Variables|Default|GetVerticesPreviousDtRow) 2) (Utilities|Array|Get(acopy) (Variables|Default|GetVerticesPreviousDtRow) 3) (Math|Vector|MakeVectorNetQuantize (.BottomSlowRightX (Utilities|Struct|BreakS_Transit3DFourVerticesOfATime _returnvalue)) (.BottomSlowRightY (Utilities|Struct|BreakS_Transit3DFourVerticesOfATime _returnvalue)) (.BottomSlowRightTimeZ (Utilities|Struct|BreakS_Transit3DFourVerticesOfATime _returnvalue)))) (Utilities|Struct|MakeCustomMeshTriangle (Math|Vector|MakeVectorNetQuantize (.BottomSlowRightX (Utilities|Struct|BreakS_Transit3DFourVerticesOfATime _returnvalue)) (.BottomSlowRightY (Utilities|Struct|BreakS_Transit3DFourVerticesOfATime _returnvalue)) (.BottomSlowRightTimeZ (Utilities|Struct|BreakS_Transit3DFourVerticesOfATime _returnvalue))) (Utilities|Array|Get(acopy) (Variables|Default|GetVerticesPreviousDtRow) 3) (Math|Vector|MakeVectorNetQuantize (.BottomSlowLeftX (Utilities|Struct|BreakS_Transit3DFourVerticesOfATime _returnvalue)) (.BottomSlowLeftY (Utilities|Struct|BreakS_Transit3DFourVerticesOfATime _returnvalue)) (.BottomSlowLeftTimeZ (Utilities|Struct|BreakS_Transit3DFourVerticesOfATime _returnvalue)))) (Utilities|Struct|MakeCustomMeshTriangle (Utilities|Array|Get(acopy) (Variables|Default|GetVerticesPreviousDtRow) 3) (Utilities|Array|Get(acopy) (Variables|Default|GetVerticesPreviousDtRow)) (Math|Vector|MakeVectorNetQuantize (.BottomSlowLeftX (Utilities|Struct|BreakS_Transit3DFourVerticesOfATime _returnvalue)) (.BottomSlowLeftY (Utilities|Struct|BreakS_Transit3DFourVerticesOfATime _returnvalue)) (.BottomSlowLeftTimeZ (Utilities|Struct|BreakS_Transit3DFourVerticesOfATime _returnvalue)))) (Utilities|Struct|MakeCustomMeshTriangle (Math|Vector|MakeVectorNetQuantize (.BottomSlowLeftX (Utilities|Struct|BreakS_Transit3DFourVerticesOfATime _returnvalue)) (.BottomSlowLeftY (Utilities|Struct|BreakS_Transit3DFourVerticesOfATime _returnvalue)) (.BottomSlowLeftTimeZ (Utilities|Struct|BreakS_Transit3DFourVerticesOfATime _returnvalue))) (Utilities|Array|Get(acopy) (Variables|Default|GetVerticesPreviousDtRow)) (Math|Vector|MakeVectorNetQuantize (.TopFastLeftX (Utilities|Struct|BreakS_Transit3DFourVerticesOfATime _returnvalue)) (.TopFastLeftY (Utilities|Struct|BreakS_Transit3DFourVerticesOfATime _returnvalue)) (.TopFastLeftTimeZ (Utilities|Struct|BreakS_Transit3DFourVerticesOfATime _returnvalue))))))
            (Variables|Default|SetVerticesPreviousDtRow (Utilities|Array|MakeArray (Math|Vector|MakeVectorNetQuantize (.TopFastLeftX (Utilities|Struct|BreakS_Transit3DFourVerticesOfATime _returnvalue)) (.TopFastLeftY (Utilities|Struct|BreakS_Transit3DFourVerticesOfATime _returnvalue)) (.TopFastLeftTimeZ (Utilities|Struct|BreakS_Transit3DFourVerticesOfATime _returnvalue))) (Math|Vector|MakeVectorNetQuantize (.TopFastRightX (Utilities|Struct|BreakS_Transit3DFourVerticesOfATime _returnvalue)) (.TopFastRightY (Utilities|Struct|BreakS_Transit3DFourVerticesOfATime _returnvalue)) (.TopFastRightTimeZ (Utilities|Struct|BreakS_Transit3DFourVerticesOfATime _returnvalue))) (Math|Vector|MakeVectorNetQuantize (.BottomSlowRightX (Utilities|Struct|BreakS_Transit3DFourVerticesOfATime _returnvalue)) (.BottomSlowRightY (Utilities|Struct|BreakS_Transit3DFourVerticesOfATime _returnvalue)) (.BottomSlowRightTimeZ (Utilities|Struct|BreakS_Transit3DFourVerticesOfATime _returnvalue))) (Math|Vector|MakeVectorNetQuantize (.BottomSlowLeftX (Utilities|Struct|BreakS_Transit3DFourVerticesOfATime _returnvalue)) (.BottomSlowLeftY (Utilities|Struct|BreakS_Transit3DFourVerticesOfATime _returnvalue)) (.BottomSlowLeftTimeZ (Utilities|Struct|BreakS_Transit3DFourVerticesOfATime _returnvalue)))))))))))

(fn GetFirstRowOfDt
  (bind _outrownames (DataTable|GetDataTableRowNames (Variables|Default|GetSB_DataTableToDraw)))
  (bind _returnvalue (Utilities|GetDataTableRow (Variables|Default|GetSB_DataTableToDraw) (Utilities|Array|Get(acopy) _outrownames))
    (:then
      (bind _output_get (Variables|Default|SetPreivousDtRow _returnvalue))
      (Variables|Default|SetVerticesPreviousDtRow (Utilities|Array|MakeArray (Math|Vector|MakeVectorNetQuantize (.TopFastLeftX (Utilities|Struct|BreakS_Transit3DFourVerticesOfATime _output_get)) (.TopFastLeftY (Utilities|Struct|BreakS_Transit3DFourVerticesOfATime _output_get)) (.TopFastLeftTimeZ (Utilities|Struct|BreakS_Transit3DFourVerticesOfATime _output_get))) (Math|Vector|MakeVectorNetQuantize (.TopFastRightX (Utilities|Struct|BreakS_Transit3DFourVerticesOfATime _output_get)) (.TopFastRightY (Utilities|Struct|BreakS_Transit3DFourVerticesOfATime _output_get)) (.TopFastRightTimeZ (Utilities|Struct|BreakS_Transit3DFourVerticesOfATime _output_get))) (Math|Vector|MakeVectorNetQuantize (.BottomSlowRightX (Utilities|Struct|BreakS_Transit3DFourVerticesOfATime _output_get)) (.BottomSlowRightY (Utilities|Struct|BreakS_Transit3DFourVerticesOfATime _output_get)) (.BottomSlowRightTimeZ (Utilities|Struct|BreakS_Transit3DFourVerticesOfATime _output_get))) (Math|Vector|MakeVectorNetQuantize (.BottomSlowLeftX (Utilities|Struct|BreakS_Transit3DFourVerticesOfATime _output_get)) (.BottomSlowLeftY (Utilities|Struct|BreakS_Transit3DFourVerticesOfATime _output_get)) (.BottomSlowLeftTimeZ (Utilities|Struct|BreakS_Transit3DFourVerticesOfATime _output_get))))))))

(fn AssignCustomMeshtoUsetoDraw
  (params (CustomMesh :type Custom%20Mesh%20Component%20Object%20Reference%20%28by%20ref%29))
  (Variables|Default|SetSB_AssignedCustomMeshComponent CustomMesh))